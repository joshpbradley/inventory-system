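; Player controller for the inventory demo that handles input for interaction, inventory and level control.
; On BeginPlay it caches the demo HUD, whose inventory UI the Tab key opens.
; E sends an interact message to whatever the pawn's interactable detection component has in view, passing the pawn along.
; R restarts the level and Enter quits the game.
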(event EventBeginPlay
  (bind _asbp_inventory_demo_hud (Utilities|Casting|CastToBP_InventoryDemoHUD (HUD|GetHUD)))
  (Variables|Default|SetHUD _asbp_inventory_demo_hud))

(event Input|KeyboardEvents|Tab
  (params (Key :type Key%20Structure :default "None"))
  (:Pressed
    (Default|OpenInventory (Variables|/Game/InventorySystem/BP_InventoryDemoHUD.BP_InventoryDemoHUD_C|GetinventoryUI (Variables|Default|GetHUD)))))

(event Input|KeyboardEvents|E
  (params (Key :type Key%20Structure :default "None"))
  (bind _self self)
  (bind _returnvalue (Pawn|GetControlledPawn _self))
  (bind _returnvalue_2 (Actor|GetComponentbyClass _returnvalue "/Game/InventorySystem/BPC_InteractableDetection.BPC_InteractableDetection_C"))
  (bind _interactableinview (Variables|/Game/InventorySystem/BPC_InteractableDetection.BPC_InteractableDetection_C|GetinteractableInView _returnvalue_2))
  (:Pressed
    (Utilities|IsValid _returnvalue_2
      (:Is%20Valid
        (Utilities|IsValid _interactableinview
          (:Is%20Valid
            (Class|BPIInteractable|Interact(Message) _interactableinview _returnvalue)))))))

(event Input|KeyboardEvents|R
  (params (Key :type Key%20Structure :default "None"))
  (:Pressed
    (Development|ExecuteConsoleCommand "Restartlevel" 0)))

(event Input|KeyboardEvents|Enter
  (params (Key :type Key%20Structure :default "None"))
  (:Pressed
    (Game|QuitGame 0 "Quit" false)))

(fn ConstructionScript)