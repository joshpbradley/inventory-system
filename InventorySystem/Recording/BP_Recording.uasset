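; BP_Recording is an inventory preview actor that stages an item in front of a SceneCaptureComponent2D.
; SetItemToRecord clears the previous item, stores the settings and inventory index, positions the camera, and shows either a static mesh or a sprite depending on is3D.
; ClearItem resets that state, camera and visuals.
; ZoomIn and ZoomOut step the camera along X, clamped to the item's zoom limits.
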(fn ConstructionScript)

(fn SetItemtoRecord
  (params (Settings :type S%20Recording%20Settings%20Structure) (inventoryIndex :type Integer))
  (Utilities|FlowControl|Sequence
    (:then_0
      (CallFunction|ClearItem))
    (:then_1
      (Variables|Default|SetisSet true)
      (Variables|Default|SetrecordingSettings Settings)
      (Variables|Default|SetinventoryIndex inventoryIndex))
    (:then_2
      (Transformation|SetRelativeLocation (Variables|Default|GetSceneCaptureComponent2D) (.cameraposition (Variables|Default|GetrecordingSettings)) false true))
    (:then_3
      (if (.is3d (Variables|Default|GetrecordingSettings))
        (Components|StaticMesh|SetStaticMesh (Variables|Default|GetStaticMesh) (.mesh (Variables|Default|GetrecordingSettings)))
        (else
          (Rendering|Components|Sprite|SetSprite (Variables|Default|GetSprite) (.sprite (Variables|Default|GetrecordingSettings))))))))

(fn ClearItem
  (Utilities|FlowControl|Sequence
    (:then_0
      (Variables|Default|SetrecordingSettings "")
      (Variables|Default|SetisSet false)
      (Variables|Default|SetinventoryIndex -1))
    (:then_1
      (Transformation|SetRelativeLocation (Variables|Default|GetSceneCaptureComponent2D) "0, 0, 0" false false))
    (:then_2
      (Rendering|Components|Sprite|SetSprite (Variables|Default|GetSprite) 0)
      (Transformation|SetRelativeRotation (Variables|Default|GetStaticMesh) "0, 0, 0" false false)
      (Components|StaticMesh|SetStaticMesh (Variables|Default|GetStaticMesh) 0))))

(fn Zoomin
  (if (> (+ (.x (Variables|/Script/Engine.SceneComponent|GetRelativeLocation (Variables|Default|GetSceneCaptureComponent2D))) (Variables|Default|GetzoomStep)) (.maxzoomcamerapos (Variables|Default|GetrecordingSettings)))
    (Transformation|SetRelativeLocation (Variables|Default|GetSceneCaptureComponent2D) (Math|Vector|MakeVector (.maxzoomcamerapos (Variables|Default|GetrecordingSettings)) 0.0 0.0) true false)
    (else
      (Transformation|AddRelativeLocation (Variables|Default|GetSceneCaptureComponent2D) (Math|Vector|MakeVector (Variables|Default|GetzoomStep) 0.0 0.0) true false))))

(fn ZoomOut
  (if (< (- (.x (Variables|/Script/Engine.SceneComponent|GetRelativeLocation (Variables|Default|GetSceneCaptureComponent2D))) (Variables|Default|GetzoomStep)) (.minzoomcamerapos (Variables|Default|GetrecordingSettings)))
    (Transformation|SetRelativeLocation (Variables|Default|GetSceneCaptureComponent2D) (Math|Vector|MakeVector (.minzoomcamerapos (Variables|Default|GetrecordingSettings)) 0.0 0.0) true false)
    (else
      (Transformation|AddRelativeLocation (Variables|Default|GetSceneCaptureComponent2D) (Math|Vector|MakeVector (* (Variables|Default|GetzoomStep) -1.0) 0.0 0.0) true false))))