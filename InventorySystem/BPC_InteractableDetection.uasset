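; Actor component in the inventory system that detects which interactable the player camera is looking at.
; Each tick it line traces forward from the camera up to InteractionDistance on a custom trace channel, ignoring its owner.
; A hit actor implementing BPI_Interactable is stored as InteractableInView, and OnUpdateInteractableDetected broadcasts true only when that actor changes.
; Otherwise it clears the reference and broadcasts false every tick.
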(event EventTick
  (params (DeltaSeconds :type Float%20%28single-precision%29))
  (bind _returnvalue (Game|GetPlayerCameraManager 0))
  (bind _returnvalue_2 (Camera|GetCameraLocation _returnvalue))
  (bind (_outhit _returnvalue_3) (Collision|LineTraceByChannel _returnvalue_2 (+ _returnvalue_2 (* (Math|Vector|GetForwardVector (Variables|/Script/Engine.PlayerCameraManager|GetTransformComponent _returnvalue)) (Variables|Default|GetinteractionDistance))) "TraceTypeQuery3" false (Utilities|Array|MakeArray (Components|GetOwner)) "None"))
  (if _returnvalue_3
    (if (Utilities|DoesObjectImplementInterface (.hitactor _outhit) "/Game/InventorySystem/BPI_Interactable.BPI_Interactable_C")
      (if (not (== (Variables|Default|GetinteractableInView) (.hitactor _outhit)))
        (Variables|Default|SetinteractableInView (.hitactor _outhit))
        (Default|CallOnUpdateInteractableDetected true))
      (else
        (Variables|Default|SetinteractableInView 0 :!label _label)
        (Default|CallOnUpdateInteractableDetected false)))
    (else
      (goto _label))))