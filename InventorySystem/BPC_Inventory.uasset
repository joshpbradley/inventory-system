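; BPC_Inventory is an inventory component that stores items in an array limited by a Capacity value.
; AddToInventory appends an item while space remains, and DeleteFromInventory removes the entry at a valid index.
; Both functions return whether they succeeded and call OnInventoryUpdate only after a successful change.
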(fn AddtoInventory
  (params (itemToAdd :type Name))
  (if (< (Utilities|Array|Length (Variables|Default|Getinventory)) (Variables|Default|Getcapacity))
    (Utilities|Array|Add (Variables|Default|Getinventory) itemToAdd)
    (Default|CallOnInventoryUpdate)
    (return true)
    (else
      (return false))))

(fn DeletefromInventory
  (params (indexToDelete :type Integer))
  (if (Math|Integer|InRange(Integer) indexToDelete 0 (Utilities|Array|Length (Variables|Default|Getinventory)) true false)
    (Utilities|Array|RemoveIndex (Variables|Default|Getinventory) indexToDelete)
    (Default|CallOnInventoryUpdate)
    (return true)
    (else
      (return false))))